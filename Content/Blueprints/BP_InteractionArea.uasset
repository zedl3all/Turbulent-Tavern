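; BP_InteractionArea is an interaction area component that relays focus changes to the actor it belongs to.
; ToggleFocus stores the Focused state and forwards it to the parent actor through an interface message.
; If the parent reports it can interact, it fetches the parent's interaction widget and shows or hides it to match focus.
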(event Custom|ToggleFocus
  (params (Focused :type Boolean))
  (Variables|Default|SetFocused Focused)
  (Class|IInteraction|InterfaceToggleFocus(Message) (Actor|GetParentActor) (Variables|Default|GetFocused))
  (bind _caninteract (Class|IInteraction|InterfaceCanInteract(Message) (Actor|GetParentActor)))
  (if _caninteract
    (bind _widgetref (Class|IInteraction|GetInteractionWidgetRef(Message) (Actor|GetParentActor)))
    (Development|SetHiddeninGame _widgetref (not (Variables|Default|GetFocused)) false)))

(fn ConstructionScript)