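; BP_Sign is an interactable crop sign that sells a fixed batch of its linked item to the player.
; Its DT_Sign row sets the mesh and price widget, which shows while the player overlaps a sphere.
; Interacting flips InteractToggle via InteractOnServer; its OnRep charges BP_EconomyManage without checking funds, adds items to player 0's inventory, then clears the toggle.
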(event OnComponentBeginOverlap(Sphere)
  (params (OverlappedComponent :type Primitive%20Component%20Object%20Reference) (OtherActor :type Actor%20Object%20Reference) (OtherComp :type Primitive%20Component%20Object%20Reference) (OtherBodyIndex :type Integer) (bFromSweep :type Boolean) (SweepResult :type Hit%20Result%20Structure%20%28by%20ref%29))
  (Utilities|Casting|CastToBP_FirstPersonCharacter OtherActor)
  (Development|SetHiddeninGame (Variables|Default|GetPrice) false false))

(event OnComponentEndOverlap(Sphere)
  (params (OverlappedComponent :type Primitive%20Component%20Object%20Reference) (OtherActor :type Actor%20Object%20Reference) (OtherComp :type Primitive%20Component%20Object%20Reference) (OtherBodyIndex :type Integer))
  (Utilities|Casting|CastToBP_FirstPersonCharacter OtherActor)
  (Development|SetHiddeninGame (Variables|Default|GetPrice) true false))

(event Custom|InteractOnServer
  (Variables|Default|SetInteract%20Toggle (not (Variables|Default|GetInteract%20Toggle))))

(event EventBeginPlay
  (bind _returnvalue (Utilities|GetDataTableRow "/Game/Blueprints/Structure/DT_Sign.DT_Sign" (Variables|Default|GetSign%20Name))
    (:then
      (Components|StaticMesh|SetStaticMesh (Variables|Default|GetStaticMesh) (.CropSign (Utilities|Struct|BreakST_Sign _returnvalue)))
      (bind _aswbp_price (Utilities|Casting|CastToWBP_Price (UserInterface|GetWidget (Variables|Default|GetPrice))))
      (Default|SetPrice _aswbp_price (.Cost (Utilities|Struct|BreakST_Sign _returnvalue))))))

(event EventInterfaceInteract
  (CallFunction|InteractonServer))

(event EventInterfaceToggleFocus
  (params (Focus :type Boolean))
  (Development|PrintString (Utilities|String|ToString(Boolean) Focus) true true "(R=1.000000,G=0.901542,B=0.000000,A=1.000000)"))

(fn ConstructionScript)

(fn OnRepInteractToggle
  (if (Variables|Default|GetInteract%20Toggle)
    ;[0.15 0.15 0.15 0.5] Get Item Data
    (bind _returnvalue (Utilities|GetDataTableRow "/Game/Blueprints/Structure/DT_Sign.DT_Sign" (Variables|Default|GetSign%20Name))
      (:then
        (bind _returnvalue_2 (Actor|GetActorOfClass "/Game/Blueprints/BP_EconomyManage.BP_EconomyManage_C"))
        (Default|SubtractMoney _returnvalue_2 (.Cost (Utilities|Struct|BreakST_Sign _returnvalue)))
        ;[0.15 0.15 0.15 0.5] Add To Player Inv
        (bind _asbp_first_person_character (Utilities|Casting|CastToBP_FirstPersonCharacter (Game|GetPlayerCharacter 0)))
        (Default|AddItem (Variables|/Game/FirstPerson/Blueprints/BP_FirstPersonCharacter.BP_FirstPersonCharacter_C|GetBP_InventoryComponent _asbp_first_person_character) (.RowName (Utilities|Struct|BreakDataTableRowHandle (.LinkedData (Utilities|Struct|BreakST_Sign _returnvalue)))) 5)
        (Variables|Default|SetInteract%20Toggle false)))))

(fn GetInteractionWidgetRef
  (return (Variables|Default|GetPress)))

(fn InterfaceCanInteract
  (return true))