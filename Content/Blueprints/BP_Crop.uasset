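; Farm plot actor where the first-person player plants seeds and harvests grown crops through an interaction interface.
; InteractOnServer flips InteractToggle, whose OnRep chooses Plant or Harvest against player index 0's inventory.
; Planting consumes the selected seed, reads data table rows, and starts a looping timer swapping growth-stage meshes.
; A countdown component, shown on sphere overlap, marks growth finished, allowing harvest to add produce.
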(event OnComponentBeginOverlap(Sphere)
  (params (OverlappedComponent :type Primitive%20Component%20Object%20Reference) (OtherActor :type Actor%20Object%20Reference) (OtherComp :type Primitive%20Component%20Object%20Reference) (OtherBodyIndex :type Integer) (bFromSweep :type Boolean) (SweepResult :type Hit%20Result%20Structure%20%28by%20ref%29))
  ;[1 1 1 0.5] Show Count Time
  (Rendering|SetVisibility (Variables|Default|GetCountTime) true false))

(event OnComponentEndOverlap(Sphere)
  (params (OverlappedComponent :type Primitive%20Component%20Object%20Reference) (OtherActor :type Actor%20Object%20Reference) (OtherComp :type Primitive%20Component%20Object%20Reference) (OtherBodyIndex :type Integer))
  ;[1 1 1 0.5] Show Count Time
  (Rendering|SetVisibility (Variables|Default|GetCountTime) false false))

(event Custom|InteractOnServer
  (Variables|Default|SetInteractToggle (not (Variables|Default|GetInteractToggle))))

(event Custom|StartGrowing
  (params (CropState :type Array%20of%20Static%20Mesh%20Object%20References) (GrownTime :type Float%20%28double-precision%29))
  ;[1 1 1 0.5] Growing
  (CallFunction|ResetCrop)
  (Variables|Default|SetCurrentIndex 0)
  (CallFunction|Grown (Variables|Default|GetCurrentCrop) CropState)
  (bind _returnvalue (Utilities|Time|SetTimerbyEvent (delegate Custom|ChangeMeshEvent) (/ GrownTime 2.0) true))
  (Variables|Default|SetGrowthTimerHandle _returnvalue))

(event Custom|ChangeMeshEvent
  ;[1 1 1 0.5] Growing
  (if (< (Variables|Default|GetCurrentIndex) (Utilities|Array|Length (stale Custom|StartGrowing CropState)))
    (CallFunction|Grown (Variables|Default|GetCurrentCrop) (stale Custom|StartGrowing CropState))
    (else
      (Utilities|Time|ClearandInvalidateTimerbyHandle (Variables|Default|GetGrowthTimerHandle))
      (Variables|Default|SetCurrentIndex 0))))

(event Custom|FinishedGrowth
  ;[0 1 0 0.5] Growth Finished
  (Variables|Default|SetFinished%20Growth true)
  (if (Variables|Default|GetIsFocused)
    (Development|SetHiddeninGame (Variables|Default|GetPress) false false)
    (Variables|Default|SetInteractToggle false)
    (else
      (Variables|Default|SetInteractToggle false))))

(event EventBeginPlay
  ;[0 1 0 0.5] Growth Finished
  (EventDispatchers|BindEventtoOnCountdownFinished (Variables|Default|GetBP_CountdownComponent) (delegate Custom|FinishedGrowth)))

(event EventInterfaceToggleFocus
  (params (Focus :type Boolean))
  (bind _output_get (Variables|Default|SetIsFocused Focus))
  (Development|PrintString (Utilities|String|ToString(Boolean) _output_get) true true "(R=1.000000,G=0.901542,B=0.000000,A=1.000000)"))

(event EventInterfaceInteract
  (CallFunction|InteractonServer))

(fn ConstructionScript)

(fn Grown
  (params (Mesh :type Static%20Mesh%20Component%20Object%20Reference) (Array :type Array%20of%20Static%20Mesh%20Object%20References))
  (Components|StaticMesh|SetStaticMesh Mesh (Utilities|Array|Get(acopy) Array (Variables|Default|GetCurrentIndex)))
  (Variables|Default|SetCurrentIndex (+ (Variables|Default|GetCurrentIndex) 1)))

(fn ResetCrop
  (bind _growthtimerhandle (Variables|Default|GetGrowthTimerHandle))
  (Components|StaticMesh|SetStaticMesh (Variables|Default|GetCurrentCrop) 0)
  (Variables|Default|SetFinished%20Growth false)
  (Variables|Default|SetPlanted false)
  (if (Utilities|Time|IsValidTimerHandle _growthtimerhandle)
    (Utilities|Time|ClearandInvalidateTimerbyHandle _growthtimerhandle)))

(fn IsSeed?
  (params (Item%20Name :type Name))
  (bind _returnvalue (Utilities|GetDataTableRow "/Game/Blueprints/Structure/DT_Items.DT_Items" Item%20Name)
    (:then
      (return (Utilities|Enum|Equal(Enum) (.ItemType (Utilities|Struct|BreakST_ItemData _returnvalue)) "NewEnumerator0")))
    (:RowNotFound
      (return false))))

(fn SetCurrentSeedfromSlot
  ;[0.15 0.15 0.15 0.5] Get Current Slot
  (bind _asbp_first_person_character (Utilities|Casting|CastToBP_FirstPersonCharacter (Game|GetPlayerCharacter 0)))
  (bind _current_slot (Default|GetCurrentSelectedItem _asbp_first_person_character))
  (bind _is_seed_ (CallFunction|IsSeed? (.ItemID (Utilities|Struct|BreakST_InventorySlot _current_slot))))
  (if _is_seed_
    (bind _returnvalue (Utilities|GetDataTableRow "/Game/Blueprints/Structure/DT_Items.DT_Items" (.ItemID (Utilities|Struct|BreakST_InventorySlot _current_slot)))
      (:then
        (Variables|Default|SetCropRowName (.RowName (Utilities|Struct|BreakDataTableRowHandle (.LinkedData (Utilities|Struct|BreakST_ItemData _returnvalue)))))
        (Default|RemoveItem (Variables|/Game/FirstPerson/Blueprints/BP_FirstPersonCharacter.BP_FirstPersonCharacter_C|GetBP_InventoryComponent _asbp_first_person_character) (.ItemID (Utilities|Struct|BreakST_InventorySlot _current_slot)) 1)))))

(fn OnRepInteractToggle
  (if (Variables|Default|GetInteractToggle)
    (if (Variables|Default|GetPlanted)
      (if (Variables|Default|GetFinished%20Growth)
        (CallFunction|Harvest)
        (Variables|Default|SetInteractToggle false))
      (else
        (CallFunction|Plant)))))

(fn Plant
  (bind _farmfield (Variables|Default|GetFarmField))
  (bind _bp_countdowncomponent (Variables|Default|GetBP_CountdownComponent))
  (bind (_min _max) (Components|StaticMesh|GetLocalBounds _farmfield))
  (bind _asbp_first_person_character (Utilities|Casting|CastToBP_FirstPersonCharacter (Game|Player|GetPlayerPawn 0)))
  (bind _current_slot (Default|GetCurrentSelectedItem _asbp_first_person_character))
  (bind _is_seed_ (CallFunction|IsSeed? (.ItemID (Utilities|Struct|BreakST_InventorySlot _current_slot))))
  (if _is_seed_
    (CallFunction|SetCurrentSeedfromSlot)
    ;[0.15 0.15 0.15 0.5] Check Has Crop NOW?
    (Utilities|IsValid (Variables|Default|GetCurrentCrop)
      (:Is%20Valid
        _)
      (:Is%20Not%20Valid
        (bind _returnvalue (AddComponent|AddStaticMeshComponent false (Math|Transform|MakeTransform (Math|Vector|MakeVector 0.0 0.0 (.z (- _max _min))) "0, 0, 0" "1.000000,1.000000,1.000000")))
        (Variables|Default|SetCurrentCrop _returnvalue)))
    (bind _returnvalue_2 (Utilities|GetDataTableRow (Variables|Default|GetDATATABLE) (Variables|Default|GetCropRowName))
      (:then
        (CallFunction|StartGrowing (.GrowthStages (Utilities|Struct|BreakST_CropData _returnvalue_2)) (.GrowthInterval (Utilities|Struct|BreakST_CropData _returnvalue_2)))
        (Variables|Default|SetPlanted true)
        (Development|SetHiddeninGame (Variables|Default|GetPress) true false)
        ;[0.15 0.15 0.15 0.5] Set Time
        (Default|SetWidget _bp_countdowncomponent (Variables|Default|GetCountTime))
        (Default|SetTotalTime _bp_countdowncomponent (.GrowthInterval (Utilities|Struct|BreakST_CropData _returnvalue_2)))
        (Default|StartCountdown _bp_countdowncomponent)
        ;[0.15 0.15 0.15 0.5] Play Sound
        (Audio|PlaySoundatLocation "/Game/Sound/Plant_Seed.Plant_Seed" (Transformation|GetActorLocation) "0, 0, 0" 1.0 1.0 0.0 0 0 0 0)))))

(fn Harvest
  (bind _growthtimerhandle (Variables|Default|GetGrowthTimerHandle))
  (Components|StaticMesh|SetStaticMesh (Variables|Default|GetCurrentCrop) 0)
  (Variables|Default|SetFinished%20Growth false)
  (Variables|Default|SetPlanted false)
  (bind _returnvalue (Utilities|GetDataTableRow "/Game/Blueprints/Structure/DT_Crops.DT_Crops" (Variables|Default|GetCropRowName))
    (:then
      (bind _asbp_first_person_character (Utilities|Casting|CastToBP_FirstPersonCharacter (Game|GetPlayerCharacter 0)))
      (Default|AddItem (Variables|/Game/FirstPerson/Blueprints/BP_FirstPersonCharacter.BP_FirstPersonCharacter_C|GetBP_InventoryComponent _asbp_first_person_character) (.RowName (Utilities|Struct|BreakDataTableRowHandle (.LinkedData (Utilities|Struct|BreakST_CropData _returnvalue)))) 4)
      ;[0.15 0.15 0.15 0.5] Play Sound
      (Audio|PlaySoundatLocation "/Game/Sound/Pickup.Pickup" (Transformation|GetActorLocation) "0, 0, 0" 1.0 1.0 0.0 0 0 0 0)
      ;[0.15 0.15 0.15 0.5] Reset Timer
      (if (Utilities|Time|IsValidTimerHandle _growthtimerhandle)
        (Utilities|Time|ClearandInvalidateTimerbyHandle _growthtimerhandle)))))

(fn GetInteractionWidgetRef
  (return (Variables|Default|GetPress)))

(fn InterfaceCanInteract
  (if (Variables|Default|GetPlanted)
    (if (Variables|Default|GetFinished%20Growth)
      (return true)
      (else
        (return false)))
    (else
      (return true))))