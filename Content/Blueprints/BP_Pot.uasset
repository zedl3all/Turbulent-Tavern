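; Cooking pot interactable that collects ingredients, cooks a matching DT_Recipes entry on a delay and yields food to the player's inventory.
; AddIngredient runs an exact array match against recipes, then StartCooking and FinishCooking set the state flags.
; Interact flips InteractToggle in a server event, which also adds hardcoded "Corn" or grants finished food.
; InteractToggle's OnRep separately moves held ingredients into the pot without checking recipes, or gives food to empty hands.
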(event OnComponentBeginOverlap(InteractZone)
  (params (OverlappedComponent :type Primitive%20Component%20Object%20Reference) (OtherActor :type Actor%20Object%20Reference) (OtherComp :type Primitive%20Component%20Object%20Reference) (OtherBodyIndex :type Integer) (bFromSweep :type Boolean) (SweepResult :type Hit%20Result%20Structure%20%28by%20ref%29))
  ;[0.01528 0.15 0.1077 0.5] Interact Zone
  (Input|EnableInput (Game|GetPlayerController 0)))

(event OnComponentEndOverlap(InteractZone)
  (params (OverlappedComponent :type Primitive%20Component%20Object%20Reference) (OtherActor :type Actor%20Object%20Reference) (OtherComp :type Primitive%20Component%20Object%20Reference) (OtherBodyIndex :type Integer))
  ;[0.01528 0.15 0.1077 0.5] Interact Zone
  (Input|DisableInput (Game|GetPlayerController 0)))

(event Custom|Interac%20on%20Server
  (Variables|Default|SetInteract%20Toggle (not (Variables|Default|GetInteract%20Toggle)))
  (if (Variables|Default|GetIsFoodReady)
    ;[0.15 0.15 0.15 0.5] Get Item Data
    (bind _returnvalue (Utilities|GetDataTableRow "/Game/Blueprints/Structure/DT_Items.DT_Items" (Variables|Default|GetCookedFood))
      (:then
        ;[0.15 0.15 0.15 0.5] Add To Player Inv
        (bind _asbp_first_person_character (Utilities|Casting|CastToBP_FirstPersonCharacter (Game|GetPlayerCharacter 0)))
        (Default|AddItem (Variables|/Game/FirstPerson/Blueprints/BP_FirstPersonCharacter.BP_FirstPersonCharacter_C|GetBP_InventoryComponent _asbp_first_person_character) (.RowName (Utilities|Struct|BreakDataTableRowHandle (.LinkedData (Utilities|Struct|BreakST_ItemData _returnvalue)))) 5)
        (Utilities|Array|Clear (Variables|Default|GetItemsInPot))
        (Variables|Default|SetIsFoodReady false)
        (Variables|Default|SetIsCooking false)))
    (else
      (CallFunction|AddIngredientEvent "Corn"))))

(event Custom|AddIngredient_Event
  (params (ItemToAdd :type Name))
  ;[0.01153 0.05832 0.15 0.5] AddIngredient_Event
  (if (not (Variables|Default|GetIsCooking))
    (Utilities|Array|Add (Variables|Default|GetItemsInPot) ItemToAdd)
    (CallFunction|CheckRecipeEvent)))

(event Custom|CheckRecipe_Event
  ;[0.15 0.125 0.02145 0.5] CheckRecipe_Event
  (bind _outrownames (DataTable|GetDataTableRowNames 0))
  (bind _array_element (Utilities|Array|ForEachLoopwithBreak _outrownames :!label _label)
    (:LoopBody
      (bind _returnvalue (Utilities|GetDataTableRow "/Game/Blueprints/Structure/DT_Recipes.DT_Recipes" _array_element)
        (:then
          (if (Utilities|Array|Identical (Variables|Default|GetItemsInPot) (.inputingredients _returnvalue))
            (CallFunction|StartCookingEvent (.cookingtime _returnvalue) (.foodname _returnvalue))
            (goto _label Break)))))))

(event Custom|StartCooking_Event
  (params (CookTime :type Float%20%28double-precision%29) (ResultItem :type Name))
  ;[0.15 0.06874 0.01567 0.5] StartCooking_Event
  (Variables|Default|SetIsCooking true)
  (Development|PrintString (Utilities|String|ToString(Float) CookTime))
  (Utilities|FlowControl|Delay CookTime)
  (CallFunction|FinishCookingEvent ResultItem))

(event Custom|FinishCooking_Event
  (params (FinalItem :type Name))
  ;[0.03037 0.15 0.03057 0.5] FinishCooking_Event
  (Variables|Default|SetCookedFood FinalItem)
  (Variables|Default|SetIsFoodReady true)
  (Development|PrintString "Your food is ready!! Press E to pick it up"))

(event EventInterfaceInteract
  (CallFunction|InteraconServer))

(event EventInterfaceToggleFocus
  (params (Focus :type Boolean))
  (Development|PrintString (Utilities|String|ToString(Boolean) Focus) true true "(R=1.000000,G=0.901542,B=0.000000,A=1.000000)"))

(fn ConstructionScript)

(fn OnRepInteractToggle
  (bind _cookedfood (Variables|Default|GetCookedFood))
  (if (Variables|Default|GetInteract%20Toggle)
    (if (Variables|Default|GetIsFoodReady)
      ;[0.15 0.15 0.15 0.5] Finished Cook
      (bind _ishandfree (CallFunction|IsHandFree))
      (if _ishandfree
        ;;[0.15 0.15 0.15 0.5] Add TO INV
        (Development|PrintString "Get The : " true true "(R=0.000000,G=0.660000,B=1.000000,A=1.000000)" 2.0 _cookedfood)
        (CallFunction|AddFoodtoInv _cookedfood)
        (Utilities|Array|Clear (Variables|Default|GetItemsInPot))
        (Variables|Default|SetIsFoodReady false)
        (Variables|Default|SetIsCooking false)
        (Variables|Default|SetInteract%20Toggle false))
      (else
        ;[0.15 0.15 0.15 0.5] Add Item In Hand To Pot
        (bind _asbp_first_person_character (Utilities|Casting|CastToBP_FirstPersonCharacter (Game|GetPlayerCharacter 0)))
        (bind _current_slot (Default|GetCurrentSelectedItem _asbp_first_person_character))
        (bind _is_ingre_ (CallFunction|IsIngredient (.ItemID (Utilities|Struct|BreakST_InventorySlot _current_slot))))
        (if _is_ingre_
          (Default|RemoveItem (Variables|/Game/FirstPerson/Blueprints/BP_FirstPersonCharacter.BP_FirstPersonCharacter_C|GetBP_InventoryComponent _asbp_first_person_character) (.ItemID (Utilities|Struct|BreakST_InventorySlot _current_slot)) 1)
          (Utilities|Array|Add (Variables|Default|GetItemsInPot) (.ItemID (Utilities|Struct|BreakST_InventorySlot _current_slot)))
          (Variables|Default|SetInteract%20Toggle false))))))

(fn AddFoodtoInv
  (params (Food :type Name))
  (bind _returnvalue (Utilities|GetDataTableRow "/Game/Blueprints/Structure/DT_Recipes.DT_Recipes" Food)
    (:then
      (bind _asbp_first_person_character (Utilities|Casting|CastToBP_FirstPersonCharacter (Game|GetPlayerCharacter 0)))
      (Default|AddItem (Variables|/Game/FirstPerson/Blueprints/BP_FirstPersonCharacter.BP_FirstPersonCharacter_C|GetBP_InventoryComponent _asbp_first_person_character) (.RowName (Utilities|Struct|BreakDataTableRowHandle (.MenuItem (Utilities|Struct|BreakS_Recipe _returnvalue)))) 1))))

(fn IsIngredient
  (params (Item :type Name))
  (bind _returnvalue (Utilities|GetDataTableRow "/Game/Blueprints/Structure/DT_Items.DT_Items" Item)
    (:then
      (return (or (Utilities|Enum|Equal(Enum) (.ItemType (Utilities|Struct|BreakST_ItemData _returnvalue)) "NewEnumerator2") (Utilities|Enum|Equal(Enum) (.ItemType (Utilities|Struct|BreakST_ItemData _returnvalue)) "NewEnumerator1"))))
    (:RowNotFound
      (return false))))

(fn IsHandFree
  (bind _asbp_first_person_character (Utilities|Casting|CastToBP_FirstPersonCharacter (Game|GetPlayerCharacter 0)))
  (bind _current_slot (Default|GetCurrentSelectedItem _asbp_first_person_character))
  (return (== (.ItemID (Utilities|Struct|BreakST_InventorySlot _current_slot)) "")))

(fn GetInteractionWidgetRef
  (return (Variables|Default|GetPress)))

(fn InterfaceCanInteract
  (return true))