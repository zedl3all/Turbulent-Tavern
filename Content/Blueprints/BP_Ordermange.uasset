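; BP_Ordermange is an order manager that creates the main HUD and periodically fills it with recipe order tickets.
; On BeginPlay it starts a looping GenerateOrder timer, with its random interval rolled only once.
; Each firing picks a random DT_Recipes row and passes it to a new WBP_OrderTicket in the HUD's OrderList.
; Generation is skipped while the list holds five or more tickets.
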(event Custom|GenerateOrder
  (if (< (Class|PanelWidget|GetChildrenCount (Variables|/Game/UserInterface/WBP_MainHUD.WBP_MainHUD_C|GetOrderList (Variables|Default|GetMyHUD))) 5)
    (bind _outrownames (DataTable|GetDataTableRowNames "/Game/Blueprints/Structure/DT_Recipes.DT_Recipes"))
    (bind _returnvalue (Utilities|GetDataTableRow "/Game/Blueprints/Structure/DT_Recipes.DT_Recipes" (.OutItem (Utilities|Array|Random _outrownames)))
      (:then
        (bind _returnvalue_2 (UserInterface|CreateWidget "/Game/UserInterface/WBP_OrderTicket.WBP_OrderTicket_C" 0 _returnvalue))
        (Class|HorizontalBox|AddChildtoHorizontalBox (Variables|/Game/UserInterface/WBP_MainHUD.WBP_MainHUD_C|GetOrderList (Variables|Default|GetMyHUD)) _returnvalue_2)))))

(event EventBeginPlay
  (bind _returnvalue (UserInterface|CreateWidget "/Game/UserInterface/WBP_MainHUD.WBP_MainHUD_C"))
  (bind _output_get (Variables|Default|SetMyHUD _returnvalue))
  (UserInterface|Viewport|AddtoViewport _output_get 0)
  (Utilities|Time|SetTimerbyEvent (delegate Custom|GenerateOrder) (Math|Random|RandomFloatinRange 5.0 1e+01) true))

(event EventTick
  (params (DeltaSeconds :type Float%20%28single-precision%29)))

(event Collision|EventActorBeginOverlap
  (params (OtherActor :type Actor%20Object%20Reference)))

(fn ConstructionScript)