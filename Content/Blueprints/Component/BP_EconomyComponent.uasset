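; Economy component that tracks a current money balance and shows it in a UI widget.
; SubtractMoney deducts a cost only when the balance covers it, while IncreaseMoney adds to it without checks.
; Both update the widget's Money text through SetMoney, and SetWidgetRef stores the widget reference and pushes the initial balance to it.
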(event EventBeginPlay)

(event EventTick
  (params (DeltaSeconds :type Float%20%28single-precision%29)))

(fn SubtractMoney
  (params (Cost :type Integer))
  (if (>= (Variables|Default|GetCurrentMoney) Cost)
    (bind _output_get (Variables|Default|SetCurrentMoney (- (Variables|Default|GetCurrentMoney) Cost)))
    (CallFunction|SetMoney _output_get)
    (return _output_get)))

(fn SetWidgetRef
  (params (Widget :type WBP%20Main%20HUD%20Object%20Reference))
  (Variables|Default|SetWidget Widget)
  (CallFunction|SetMoney (Variables|Default|GetCurrentMoney)))

(fn SetMoney
  (params (NewMoney :type Integer))
  (Variables|/Script/UMG.TextBlock|SetText (Variables|/Game/UserInterface/WBP_MainHUD.WBP_MainHUD_C|GetMoney (Variables|Default|GetWidget)) (Utilities|Text|ToText(Integer) NewMoney)))

(fn IncreaseMoney
  (params (Money :type Integer))
  (bind _output_get (Variables|Default|SetCurrentMoney (+ Money (Variables|Default|GetCurrentMoney))))
  (CallFunction|SetMoney _output_get)
  (return _output_get))