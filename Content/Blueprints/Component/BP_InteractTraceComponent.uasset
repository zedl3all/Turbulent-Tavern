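; Player interaction component that finds the BP_InteractionArea under the camera and triggers interaction with it.
; Each tick it line-traces forward on Visibility, toggling focus on interaction areas as the hit actor changes or is lost.
; TryToInteract passes a focused area with no positive InteractDuration to InteractOnServer, which sends an interface message to its parent actor.
; Areas with a positive duration get no further handling here.
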(event Custom|TryToInteract
  (params (In :type Boolean))
  (if In
    (if (Variables|Default|GetIsTraceInteractionArea)
      (bind _output_get (Variables|Default|SetInteract%20Duration (Variables|/Game/Blueprints/BP_InteractionArea.BP_InteractionArea_C|GetInteractDuration (Variables|Default|GetFocusedInteractionArea))))
      (if (not (> _output_get 0.0))
        (CallFunction|InteractonServer (Variables|Default|GetFocusedInteractionArea))))))

(event Custom|InteractOnServer
  (params (InteractionArea :type BP%20Interaction%20Area%20Object%20Reference))
  (Class|IInteraction|InterfaceInteract(Message) (Actor|GetParentActor InteractionArea)))

(event EventTick
  (params (DeltaSeconds :type Float%20%28single-precision%29))
  (CallFunction|Trace))

(fn Trace
  (bind _returnvalue (Game|GetPlayerCameraManager 0))
  (bind _returnvalue_2 (Transformation|GetActorLocation _returnvalue))
  (bind (_outhit _returnvalue_3) (Collision|LineTraceByChannel _returnvalue_2 (+ _returnvalue_2 (* (Math|Vector|GetForwardVector (Transformation|GetActorRotation _returnvalue)) (Variables|Default|GetLength))) "TraceTypeQuery1" false 0 "None"))
  (if _returnvalue_3
    (if (!= (Variables|Default|GetFocusedActor) (.HitActor (Collision|BreakHitResult _outhit)))
      (Variables|Default|SetFocusedActor (.HitActor (Collision|BreakHitResult _outhit)))
      (CallFunction|TraceInteractionArea (== (Utilities|GetClass (.HitActor (Collision|BreakHitResult _outhit))) "/Game/Blueprints/BP_InteractionArea.BP_InteractionArea_C")))
    (else
      (CallFunction|TraceInteractionArea false))))

(fn TraceInteractionArea
  (params (Trace :type Boolean))
  (if Trace
    (if (Variables|Default|GetIsTraceInteractionArea)
      ;[0.15 0.15 0.15 0.5] Focus Another
      (Default|ToggleFocus (Variables|Default|GetFocusedInteractionArea) false))
    ;[0.15 0.15 0.15 0.5] If Trace & If not Focused
    (bind _asbp_interaction_area (Utilities|Casting|CastToBP_InteractionArea (Variables|Default|GetFocusedActor)))
    (bind _output_get (Variables|Default|SetFocusedInteractionArea _asbp_interaction_area))
    (Default|ToggleFocus _output_get true)
    (Variables|Default|SetIsTraceInteractionArea true)
    (elif (Variables|Default|GetIsTraceInteractionArea)
      ;[0.15 0.15 0.15 0.5] Don't Look
      (Variables|Default|SetIsTraceInteractionArea false)
      (Default|ToggleFocus (Variables|Default|GetFocusedInteractionArea) false)
      (Variables|Default|SetFocusedActor 0)
      (Variables|Default|SetFocusedInteractionArea 0))))