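; Inventory component that stores items as ItemID and Quantity slots, with functions to add, remove and query them.
; Each add, remove or quantity lookup validates the ItemID against DT_Items, which also supplies MaxStack.
; AddItem increases the first matching slot, failing if it is full, and creates a slot only for unheld items while under MaxInventorySize.
; RemoveItem decrements or deletes the slot, and successful changes fire OnInventoryChanged.
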(event EventBeginPlay)

(event EventTick
  (params (DeltaSeconds :type Float%20%28single-precision%29)))

(fn AddItem
  (params (ItemID :type Name) (Amount :type Integer))
  ;[0.15 0.15 0.15 0.5] Check Amount
  (if (> Amount 0)
    ;[0.15 0.15 0.15 0.5] Get Data Table
    (bind _returnvalue (Utilities|GetDataTableRow "/Game/Blueprints/Structure/DT_Items.DT_Items" ItemID)
      (:then
        (bind _output_get (LocalVariables|SetMax%20Stack (.MaxStack (Utilities|Struct|BreakST_ItemData _returnvalue))))
        ;[0.15 0.15 0.15 0.5] Space Left & RemainingAmount
        (LocalVariables|SetSpaceLeft%20 (- _output_get Amount))
        (LocalVariables|SetRemainingAmount%20 Amount)
        ;[0.15 0.15 0.15 0.5] Loop Check Current Stack
        (for (_array_element _array_index) (Variables|Default|GetInventory)
          (if (== (.ItemID (Utilities|Struct|BreakST_InventorySlot _array_element)) ItemID)
            ;[0.15 0.15 0.15 0.5] Same Item
            (if (< (.Quantity (Utilities|Struct|BreakST_InventorySlot _array_element)) (LocalVariables|GetMax%20Stack))
              ;[0.15 0.15 0.15 0.5] New Quantity
              (bind _structout (Utilities|Struct|SetmembersinST_InventorySlot _array_element (+ (Math|Integer|Min(Integer) (LocalVariables|GetSpaceLeft%20) (LocalVariables|GetRemainingAmount%20)) (.Quantity (Utilities|Struct|BreakST_InventorySlot _array_element)))))
              (Utilities|Array|SetArrayElem (Variables|Default|GetInventory) _array_index _structout)
              (LocalVariables|SetIS%20ADD true)
              (Default|CallOnInventoryChanged)
              (return true)
              (else
                (return false)))))
        ;[0.15 0.15 0.15 0.5] Check Is ADD?
        (if (not (LocalVariables|GetIS%20ADD))
          ;[0.15 0.15 0.15 0.5] Add new Slot
          (if (< (Variables|Default|GetCurrent%20InventorySize) (Variables|Default|GetMax%20InventorySize))
            (Utilities|Array|Add (Variables|Default|GetInventory) (Utilities|Struct|MakeST_InventorySlot ItemID (LocalVariables|GetRemainingAmount%20)))
            (Math|Integer|IncrementInt (Variables|Default|GetCurrent%20InventorySize)
              (:%20%20
                (Default|CallOnInventoryChanged)
                (return true)))
            (else
              (return false)))))
      (:RowNotFound
        (return false)))
    (else
      (return false))))

(fn RemoveItem
  (params (ItemID :type Name) (Amount :type Integer))
  ;[0.15 0.15 0.15 0.5] Check Is That Item In Game?
  (Utilities|GetDataTableRow "/Game/Blueprints/Structure/DT_Items.DT_Items" ItemID
    (:then
      ;[0.15 0.15 0.15 0.5] Check Has Item?
      (bind _has (CRUD|HasItem ItemID))
      (if _has
        ;[0.15 0.15 0.15 0.5] Loop Check Item In Inv
        (for (_array_element _array_index) (Variables|Default|GetInventory)
          (if (== (.ItemID (Utilities|Struct|BreakST_InventorySlot _array_element)) ItemID)
            (if (<= (- (.Quantity (Utilities|Struct|BreakST_InventorySlot _array_element)) Amount) 0)
              ;[0.15 0.15 0.15 0.5] IF <= 0
              (Utilities|Array|RemoveItem (Variables|Default|GetInventory) _array_element)
              (Math|Integer|DecrementInt (Variables|Default|GetCurrent%20InventorySize)
                (:%20%20
                  (Default|CallOnInventoryChanged)
                  (return true)))
              (else
                ;[0.15 0.15 0.15 0.5] IF > 0
                (bind _structout (Utilities|Struct|SetmembersinST_InventorySlot _array_element (- (.Quantity (Utilities|Struct|BreakST_InventorySlot _array_element)) Amount)))
                (Utilities|Array|SetArrayElem (Variables|Default|GetInventory) _array_index _structout)
                (Default|CallOnInventoryChanged)
                (return true)))))
        (return false)
        (else
          (return false))))))

(fn HasItem
  (params (ItemID :type Name))
  ;[0.15 0.15 0.15 0.5] Check Is That Item In Game?
  (Utilities|GetDataTableRow "/Game/Blueprints/Structure/DT_Items.DT_Items" ItemID
    (:then
      ;[0.15 0.15 0.15 0.5] Loop Check Item In Inv
      (for _array_element (Variables|Default|GetInventory)
        (if (== (.ItemID (Utilities|Struct|BreakST_InventorySlot _array_element)) ItemID)
          (return true)))
      (return false))
    (:RowNotFound
      (return false))))

(fn GetItemQuantity
  (params (ItemID :type Name))
  ;[0.15 0.15 0.15 0.5] Check Is That Item In Game?
  (Utilities|GetDataTableRow "/Game/Blueprints/Structure/DT_Items.DT_Items" ItemID
    (:then
      ;[0.15 0.15 0.15 0.5] Check Has Item?
      (bind _has (CRUD|HasItem ItemID))
      (if _has
        ;[0.15 0.15 0.15 0.5] Loop Check Item In Inv
        (for _array_element (Variables|Default|GetInventory)
          (if (== (.ItemID (Utilities|Struct|BreakST_InventorySlot _array_element)) ItemID)
            (return (.Quantity (Utilities|Struct|BreakST_InventorySlot _array_element)))
            (else
              (return 0))))
        (else
          (return 0))))))

(fn GetInventory
  (return (Variables|Default|GetInventory)))

(fn GetSlot
  (params (Index :type Integer))
  (return (Utilities|Array|Get(acopy) (Variables|Default|GetInventory) Index)))