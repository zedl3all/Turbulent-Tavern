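; CP_Item is a world pickup actor that adds one of its item to the first-person character's inventory.
; On BeginPlay it looks up ItemName in DT_Items, sets the static mesh, enables physics and sizes the collision sphere to the mesh bounds.
; When the character overlaps the sphere, it passes the row's ItemID to BPInventoryComponent and destroys itself.
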(event OnComponentBeginOverlap(Collision)
  (params (OverlappedComponent :type Primitive%20Component%20Object%20Reference) (OtherActor :type Actor%20Object%20Reference) (OtherComp :type Primitive%20Component%20Object%20Reference) (OtherBodyIndex :type Integer) (bFromSweep :type Boolean) (SweepResult :type Hit%20Result%20Structure%20%28by%20ref%29))
  (bind _asbp_first_person_character (Utilities|Casting|CastToBP_FirstPersonCharacter OtherActor))
  (Default|AddItem (Variables|/Game/FirstPerson/Blueprints/BP_FirstPersonCharacter.BP_FirstPersonCharacter_C|GetBP_InventoryComponent _asbp_first_person_character) (.ItemID (Utilities|Struct|BreakST_ItemData (stale EventBeginPlay _returnvalue))) 1)
  (Actor|DestroyActor))

(event EventBeginPlay
  (bind _mesh (Variables|Default|GetMesh))
  (bind _returnvalue (Utilities|GetDataTableRow "/Game/Blueprints/Structure/DT_Items.DT_Items" (Variables|Default|GetItemName))
    (:then
      (Components|StaticMesh|SetStaticMesh _mesh (.StaticMesh (Utilities|Struct|BreakST_ItemData _returnvalue)))
      (Physics|SetSimulatePhysics _mesh true)
      (Components|Sphere|SetSphereRadius (Variables|Default|GetCollision) (.sphereradius (StaticMesh|GetBounds (.StaticMesh (Utilities|Struct|BreakST_ItemData _returnvalue)))) true))))

(fn ConstructionScript)